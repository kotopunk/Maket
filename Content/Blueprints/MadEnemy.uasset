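; MadEnemy is an enemy Blueprint that takes damage and is removed from the world when its health runs out.
; On AnyDamage it prints a "Hello" debug string, then, unless already dead, subtracts the damage from EnemyHealth.
; When health is no longer above zero, it sets IsDead and destroys the actor.
; BeginPlay, Tick, overlap and the construction script hold no logic.
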(event `self.ReceiveAnyDamage`
  (params (Damage :type "Float (single-precision)") (DamageType :type "DamageType Object Reference") (InstigatedBy :type "Controller Object Reference") (DamageCauser :type "Actor Object Reference"))
  (`KismetSystemLibrary.PrintString` "Hello")
  (if (not (`self.IsDead`))
    (set `self.EnemyHealth` (- (`self.EnemyHealth`) Damage))
    (if (not (> (`self.EnemyHealth`) 0.0))
      (set `self.IsDead` true)
      (`self.K2_DestroyActor`))))

(fn `UserConstructionScript`)